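; Actor component that simulates N-body gravity and moves its owner, either for all bodies or only the player pawn.
; While IsZeroG is set, Tick sums pulls from other "PhysicsObject"-tagged actors' gravity components into acceleration, ignoring own mass.
; CalculateFg uses inverse-distance rather than inverse-square falloff for gameplay feel.
; Acceleration integrates into Speed for a swept world offset, and blocking hits zero the speed.
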(event EventBeginPlay
  ;[0.3455 0.4249 0.6823] Begin Play
  (Utilities|Array|Clear (Variables|Movement|GetListForces)) ; Make sure array is empty
  (Variables|Default|SetSelfRef (Components|GetOwner)) ; Set up reference to the actor this component is attached to
  (Variables|Movement|SetSpeed (Variables|Movement|GetInitialSpeed)) ; Set initial speed
)

(event EventTick
  (params (DeltaSeconds :type Float%20%28single-precision%29))
  (bind _returnvalue (Utilities|Time|GetWorldDeltaSeconds))
  ;[0.3455 0.4249 0.6823] Find out what needs to be calculated
  (if (Variables|Default|GetbIsZeroG)
    (Variables|Movement|SetNetForce "0, 0, 0") ; Because Force needs to be recalculated each tick
    (if (Variables|Default|GetbPlanetsAttractEachOther) ; If False, only player is affected by gravity
      (bind _outactors (Actor|GetAllActorswithTag "PhysicsObject" :!label _label)) ; All actors that can have gravity have this tag
      (bind _output_get (Variables|Gravity|SetListPhysicsObjects _outactors)) ; Add all of those to the list
      ;[0.3455 0.4249 0.6823] Run calculations for each actor in the list
      (for _array_element _output_get
        (if (not (== _array_element (Variables|Default|GetSelfRef))) ; Don't do calculations with self
          (bind _output_get_2 (Variables|Gravity|SetMassOther (Variables|AC_GravityComponent_C|GetMassSelf (Actor|GetComponentbyClass _array_element "AC_GravityComponent_C")))) ; Set object's mass as MassOther for calculation
          (bind _force (Utilities|CalculateFg (Variables|Gravity|GetGravityConstant) _output_get_2 (- (Transformation|GetActorLocation _array_element) (Transformation|GetActorLocation (Variables|Default|GetSelfRef)))) ; Run gravity calculation macro
            (:Output
              (CallFunction|AddForcetoArray _force (Variables|Default|GetSelfRef)) ; Add a force to the array ListForces
            ))))
      (elif (== (Utilities|GetClass (Variables|Default|GetSelfRef)) (Utilities|GetClass (Game|Player|GetPlayerPawn 0))) ; If this object is not the player, return False
        (goto _label)
        (else
          _)))
    ;[0.3455 0.4249 0.6823] Calculate net force, acceleration and speed.
    ;;[0.6823 0.2878 0.3362] Calculate net force from list of forces
    (for _array_element_2 (Variables|Movement|GetListForces) ; Run calculation for each force on self
      (Variables|Movement|SetNetForce (+ _array_element_2 (Variables|Movement|GetNetForce))) ; Add each force in the array to each other to get the net force
    )
    ;;[0.6823 0.2878 0.3362] Calculate acceleration vector from net force
    (bind _output_get_3 (Variables|Movement|SetAcceleration (* (Math|Vector|Normalize (Variables|Movement|GetNetForce)) (Math|Vector|VectorLength (Variables|Movement|GetNetForce))))) ; Set new acceleration variable
    ;;[0.6823 0.2878 0.3362] Update speed and apply movement
    (bind _output_get_4 (Variables|Movement|SetSpeed (+ (* _output_get_3 _returnvalue) (Variables|Movement|GetSpeed)))) ; Set new speed variable
    (bind _sweephitresult (Transformation|AddActorWorldOffset (Variables|Default|GetSelfRef) (* _output_get_4 _returnvalue) true)) ; Move the object
    (Utilities|Array|Clear (Variables|Movement|GetListForces)) ; Clear list at the end of each tick
    (if (.bblockinghit _sweephitresult)
      (Variables|Movement|SetSpeed "0, 0, 0"))))