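; Blueprint function library of shared helpers for zero-gravity player and physics movement in an Outer Wilds-style controller.
; It appends forces to a target's gravity component and toggles zero-G on either the player pawn or every actor tagged PhysicsObject.
; Other helpers rotate the player's tagged direction arrow and return references to the player's controller, space movement and gravity components, camera and arrow.
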(fn AddForcetoArray
  (params (Force :type Vector) (Target :type Actor%20Object%20Reference))
  (Utilities|Array|Add (Variables|/Game/OuterWildsPlayerController/OuterWildsPlayerController/Blueprints/AC_GravityComponent.AC_GravityComponent_C|GetListForces (Actor|GetComponentbyClass Target "/Game/OuterWildsPlayerController/OuterWildsPlayerController/Blueprints/AC_GravityComponent.AC_GravityComponent_C")) Force) ; Add Force to a list of all forces on self
)

(fn Enable/DisableZero-G
  (params (PlayerOnly :type Boolean) (NewValue :type Boolean))
  (if PlayerOnly
    (Variables|/Game/OuterWildsPlayerController/OuterWildsPlayerController/Blueprints/AC_GravityComponent.AC_GravityComponent_C|SetbIsZeroG (Actor|GetComponentbyClass (Game|Player|GetPlayerPawn 0) "/Game/OuterWildsPlayerController/OuterWildsPlayerController/Blueprints/AC_GravityComponent.AC_GravityComponent_C") NewValue)
    (else
      (bind _outactors (Actor|GetAllActorswithTag 0 "PhysicsObject"))
      (for _array_element _outactors
        (Variables|/Game/OuterWildsPlayerController/OuterWildsPlayerController/Blueprints/AC_GravityComponent.AC_GravityComponent_C|SetbIsZeroG (Actor|GetComponentbyClass _array_element "/Game/OuterWildsPlayerController/OuterWildsPlayerController/Blueprints/AC_GravityComponent.AC_GravityComponent_C") NewValue)))))

(fn RotateDirectionArrow
  (params (Rotation%20X%20%28Roll%29 :type Float%20%28double-precision%29) (Rotation%20Y%20%28%20Pitch%29 :type Float%20%28double-precision%29) (Rotation%20Z%20%28Yaw%29 :type Float%20%28double-precision%29))
  (Transformation|AddLocalRotation (Utilities|Array|Get(acopy) (Actor|GetComponentsbyTag (Game|Player|GetPlayerPawn 0) "/Script/Engine.ArrowComponent" "DirectionArrow")) (Math|Rotator|MakeRotator Rotation%20X%20%28Roll%29 Rotation%20Y%20%28%20Pitch%29 Rotation%20Z%20%28Yaw%29) false false))

(fn GetPlayerReferences
  (bind _returnvalue (Game|Player|GetPlayerPawn 0))
  (return (Actor|GetComponentbyClass (Game|GetPlayerController 0) "/Game/OuterWildsPlayerController/OuterWildsPlayerController/Blueprints/AC_SpaceMovementComponent.AC_SpaceMovementComponent_C") (Actor|GetComponentbyClass _returnvalue "/Game/OuterWildsPlayerController/OuterWildsPlayerController/Blueprints/AC_GravityComponent.AC_GravityComponent_C") (Utilities|Array|Get(acopy) (Actor|GetComponentsbyTag _returnvalue "/Script/Engine.ArrowComponent" "DirectionArrow")) (Actor|GetComponentbyClass (Game|Player|GetPlayerPawn 0) "/Script/Engine.CameraComponent") (Game|GetPlayerController 0)))