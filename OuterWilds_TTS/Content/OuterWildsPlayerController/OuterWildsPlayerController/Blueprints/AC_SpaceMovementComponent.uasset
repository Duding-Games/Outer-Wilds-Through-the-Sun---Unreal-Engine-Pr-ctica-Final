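; Actor component for jetpack space movement and free-look rotation in an Outer Wilds-style player controller.
; Move, up/down and brake inputs add forces to the player, using camera axes for thrust and normalized velocity for braking.
; Look input rotates a DirectionArrow, with a held roll input swapping yaw for roll.
; Each tick, the camera follows the arrow through LerpCameraToArrow in zero-G; otherwise the arrow is synced to the camera.
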(event Input|EnhancedActionEvents|EnhancedInputActionIA_Move
  (params (ActionValue :type Vector%202D%20Structure) (ElapsedSeconds :type Float%20%28double-precision%29) (TriggeredSeconds :type Float%20%28double-precision%29) (InputAction :type Input%20Action%20Object%20Reference :default "/Game/OuterWildsPlayerController/OuterWildsPlayerController/Controller/IA_Move.IA_Move"))
  (bind _cameraref (Variables|Default|GetCameraRef))
  ;[0.3455 0.4249 0.6823] Jetpack Movement
  ;;[0.6823 0.2878 0.3362] Jetpack movement: Left Joystick
  (CallFunction|AddForcetoArray (* (+ (* (.x ActionValue) (Math|Vector|GetRightVector _cameraref)) (* (Math|Vector|GetForwardVector _cameraref) (.y ActionValue))) (Variables|/Game/OuterWildsPlayerController/OuterWildsPlayerController/Blueprints/Data/PDA_CharacterVariables.PDA_CharacterVariables_C|GetMoveAcceleration (Variables|Default|GetCharacterVariables))) (Game|Player|GetPlayerPawn 0)))

(event Input|EnhancedActionEvents|EnhancedInputActionIA_Look
  (params (ActionValue :type Vector%202D%20Structure) (ElapsedSeconds :type Float%20%28double-precision%29) (TriggeredSeconds :type Float%20%28double-precision%29) (InputAction :type Input%20Action%20Object%20Reference :default "/Game/OuterWildsPlayerController/OuterWildsPlayerController/Controller/IA_Look.IA_Look"))
  (bind _returnvalue (Utilities|Time|GetWorldDeltaSeconds))
  (bind _charactervariables (Variables|Default|GetCharacterVariables))
  (bind _rotationspeed (Variables|/Game/OuterWildsPlayerController/OuterWildsPlayerController/Blueprints/Data/PDA_CharacterVariables.PDA_CharacterVariables_C|GetRotationSpeed _charactervariables))
  (bind _returnvalue_2 (* (.y ActionValue) _returnvalue _rotationspeed))
  ;[0.3455 0.4249 0.6823] Camera Rotation
  ;;[0.6823 0.2878 0.3362] Rotation: apply local rotation to DirectionArrow
  (if (Variables|Default|GetbIsRolling) ; Is the player holding Left Shoulder?
    (CallFunction|RotateDirectionArrow (* (Variables|/Game/OuterWildsPlayerController/OuterWildsPlayerController/Blueprints/Data/PDA_CharacterVariables.PDA_CharacterVariables_C|GetRollSpeed (Variables|Default|GetCharacterVariables)) (Utilities|Time|GetWorldDeltaSeconds) (.x ActionValue)) _returnvalue_2 0.0) ; Apply rotation to DirectionArrow
    (else
      (CallFunction|RotateDirectionArrow 0.0 _returnvalue_2 (* _rotationspeed _returnvalue (.x ActionValue))) ; Apply rotation to DirectionArrow
    )))

(event Input|EnhancedActionEvents|EnhancedInputActionIA_UpDown
  (params (ActionValue :type Float%20%28double-precision%29) (ElapsedSeconds :type Float%20%28double-precision%29) (TriggeredSeconds :type Float%20%28double-precision%29) (InputAction :type Input%20Action%20Object%20Reference :default "/Game/OuterWildsPlayerController/OuterWildsPlayerController/Controller/IA_UpDown.IA_UpDown"))
  ;[0.3455 0.4249 0.6823] Jetpack Movement
  ;;[0.6823 0.2878 0.3362] Jetpack movement: Left and Right Triggers
  (CallFunction|AddForcetoArray (* (* ActionValue (Math|Vector|GetUpVector (Variables|Default|GetCameraRef))) (Variables|/Game/OuterWildsPlayerController/OuterWildsPlayerController/Blueprints/Data/PDA_CharacterVariables.PDA_CharacterVariables_C|GetUpDownAcceleration (Variables|Default|GetCharacterVariables))) (Game|Player|GetPlayerPawn 0)))

(event Input|EnhancedActionEvents|EnhancedInputActionIA_Brake
  (params (ActionValue :type Boolean) (ElapsedSeconds :type Float%20%28double-precision%29) (TriggeredSeconds :type Float%20%28double-precision%29) (InputAction :type Input%20Action%20Object%20Reference :default "/Game/OuterWildsPlayerController/OuterWildsPlayerController/Controller/IA_Brake.IA_Brake"))
  ;[0.3455 0.4249 0.6823] Jetpack Movement
  ;;[0.6823 0.2878 0.3362] Jetpack movement: Match Velocity / Braking
  (CallFunction|AddForcetoArray (* (Math|Vector|Normalize (Variables|/Game/OuterWildsPlayerController/OuterWildsPlayerController/Blueprints/AC_GravityComponent.AC_GravityComponent_C|GetSpeed (Variables|Default|GetPhysicsRef))) (Variables|/Game/OuterWildsPlayerController/OuterWildsPlayerController/Blueprints/Data/PDA_CharacterVariables.PDA_CharacterVariables_C|GetBrakeAcceleration (Variables|Default|GetCharacterVariables))) (Game|Player|GetPlayerPawn 0)))

(event Input|EnhancedActionEvents|EnhancedInputActionIA_Roll
  (params (ActionValue :type Boolean) (ElapsedSeconds :type Float%20%28double-precision%29) (TriggeredSeconds :type Float%20%28double-precision%29) (InputAction :type Input%20Action%20Object%20Reference :default "/Game/OuterWildsPlayerController/OuterWildsPlayerController/Controller/IA_Roll.IA_Roll"))
  ;[0.3455 0.4249 0.6823] Camera Rotation
  ;;[0.6823 0.2878 0.3362] Update Roll
  (:Started
    (Variables|Default|SetbIsRolling true))
  (:Completed
    (Variables|Default|SetbIsRolling false)))

(event EventBeginPlay
  (bind (_spacemovementcomponent _playergravitycomponent _directionarrow _playercamera) (CallFunction|GetPlayerReferences))
  ;[0.3455 0.4249 0.6823] Set up references to player components
  (Variables|Default|SetSelfRef (Game|Player|GetPlayerPawn 0)) ; Reference to player actor
  (Variables|Default|SetPhysicsRef _playergravitycomponent) ; Reference to player's GravityComponent
  (Variables|Default|SetArrowRef _directionarrow) ; Reference to player's DirectionArrow
  (Variables|Default|SetCameraRef _playercamera) ; Reference to CameraComponent
)

(event EventTick
  (params (DeltaSeconds :type Float%20%28single-precision%29))
  (bind (_newcamerarotation _camerarotation) (Utilities|LerpCameratoArrow))
  ;[0.3455 0.4249 0.6823] Camera Rotation
  ;;[0.6823 0.2878 0.3362] Apply camera rotations
  (if (Variables|/Game/OuterWildsPlayerController/OuterWildsPlayerController/Blueprints/AC_GravityComponent.AC_GravityComponent_C|GetbIsZeroG (Variables|Default|GetPhysicsRef))
    (Transformation|SetRelativeRotation (Variables|Default|GetCameraRef) _newcamerarotation false false) ; Set camera rotation to the result of the lerp
    (else
      (Transformation|SetWorldRotation (Variables|Default|GetArrowRef) _camerarotation false false) ; Prevent ArrowRef from moving
    )))