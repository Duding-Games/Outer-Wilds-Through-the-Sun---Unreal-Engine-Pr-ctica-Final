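; Trigger actor that shows its configured text on screen while the player overlaps its Trigger component.
; On overlap it removes every other top-level WBP_ScreenText, then creates or reuses its saved widget and updates the text, so only one message shows.
; When the player leaves, a retriggerable delay of TimeToDelete runs before removing and clearing the widget; re-entering does not cancel it.
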(event OnComponentBeginOverlap(Trigger)
  (params (OverlappedComponent :type Primitive%20Component%20Object%20Reference) (OtherActor :type Actor%20Object%20Reference) (OtherComp :type Primitive%20Component%20Object%20Reference) (OtherBodyIndex :type Integer) (bFromSweep :type Boolean) (SweepResult :type Hit%20Result%20Structure%20%28by%20ref%29))
  (Utilities|Casting|CastToBP_Player OtherActor)
  (bind _foundwidgets (Widget|GetAllWidgetsOfClass "/Game/Widgets/WBP_ScreenText.WBP_ScreenText_C" true))
  (for _array_element _foundwidgets
    (if (!= _array_element (Variables|Default|GetSavedWidget))
      (Widget|RemovefromParent _array_element)))
  (if (Utilities|IsValid (Variables|Default|GetSavedWidget))
    _
    (else
      (bind _returnvalue (UserInterface|CreateWidget "/Game/Widgets/WBP_ScreenText.WBP_ScreenText_C"))
      (bind _output_get (Variables|Default|SetSavedWidget _returnvalue))
      (UserInterface|Viewport|AddtoViewport _output_get 0)))
  (Default|UpdateText (Variables|Default|GetSavedWidget) (Variables|Default|GetTextToShow)))

(event OnComponentEndOverlap(Trigger)
  (params (OverlappedComponent :type Primitive%20Component%20Object%20Reference) (OtherActor :type Actor%20Object%20Reference) (OtherComp :type Primitive%20Component%20Object%20Reference) (OtherBodyIndex :type Integer))
  (Utilities|Casting|CastToBP_Player OtherActor)
  (Utilities|FlowControl|RetriggerableDelay (Variables|Default|GetTimeToDelete))
  (Utilities|IsValid (Variables|Default|GetSavedWidget)
    (:Is%20Valid
      (Widget|RemovefromParent (Variables|Default|GetSavedWidget))
      (Variables|Default|SetSavedWidget 0))))

(fn ConstructionScript)