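; BP_FinalDoor is a door blocked by a Shield that drops once enough BP_FinalDoorButton presses are registered.
; RegisterPressedButton stores the latest button's time as CooldownTime, counts presses and calls TurnOffShield when NeededButtons is reached.
; TurnOffShield hides the shield and disables its collision; with a positive cooldown it restores both after a delay, zeroes the count and re-arms every button in the level.
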(event Custom|TurnOffShield
  (bind _shield (Variables|Default|GetShield))
  (bind _cooldowntime (Variables|Default|GetCooldownTime))
  (bind _shield_2 (Variables|Default|GetShield))
  (Rendering|SetVisibility _shield false false)
  (Collision|SetCollisionEnabled _shield "NoCollision")
  (if (> _cooldowntime 0.0)
    (Utilities|FlowControl|Delay _cooldowntime)
    (Rendering|SetVisibility _shield_2 true false)
    (Collision|SetCollisionEnabled _shield_2 "QueryAndPhysics")
    (Variables|Default|SetPressedButtons 0)
    (bind _outactors (Actor|GetAllActorsOfClass "/Game/Blueprints/BP_FinalDoorButton.BP_FinalDoorButton_C"))
    (for _array_element _outactors
      (Variables|/Game/Blueprints/BP_FinalDoorButton.BP_FinalDoorButton_C|SetAlreadyPressed _array_element false))))

(fn ConstructionScript)

(fn RegisterPressedButton
  (params (ButtonTime :type Float%20%28double-precision%29))
  (Variables|Default|SetCooldownTime ButtonTime)
  (Math|Integer|IncrementInt (Variables|Default|GetPressedButtons)
    (:%20%20
      (if (>= (Variables|Default|GetPressedButtons) (Variables|Default|GetNeededButtons))
        (CallFunction|TurnOffShield)
        (return)))))